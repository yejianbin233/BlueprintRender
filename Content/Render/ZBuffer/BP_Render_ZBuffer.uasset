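; BP_Render_ZBuffer renders the Cube mesh triangle by triangle into a Z-buffer render target, once at BeginPlay.
; It copies the mesh into a procedural mesh, transforms vertices into camera space, and perspective-projects them with WorldToScreen using FOV and target aspect.
; Each triangle passes screen positions, UVs and inverse depths to a dynamic M_ZBuffer material drawn on the canvas.
; After each triangle, M_ZBuffer is drawn into RT_ZBufferCopy.
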(event EventBeginPlay
  (Rendering|ClearRenderTarget2D "/Game/Render/ZBuffer/RT_ZBuffer.RT_ZBuffer")
  (Rendering|ClearRenderTarget2D "/Game/Render/ZBuffer/RT_ZBufferCopy.RT_ZBufferCopy")
  (Variables|Default|SetStatic%20Mesh%20Relative%20Transform (Transformation|GetRelativeTransform (Variables|Default|GetCube)))
  (bind _returnvalue (Rendering|Material|CreateDynamicMaterialInstance "/Game/Render/ZBuffer/M_ZBuffer.M_ZBuffer" "None" "None" :!class /Script/Engine.KismetMaterialLibrary))
  (Variables|Default|SetZ%20Buffer%20Depth%20Painter _returnvalue)
  (Class|KismetProceduralMeshLibrary|CopyProceduralMeshfromStaticMeshComponent (Variables|Default|GetCube) 0 (Variables|Default|GetProceduralMesh) false)
  (bind (_vertices _triangles _normals _uvs) (Class|KismetProceduralMeshLibrary|GetSectionfromProceduralMesh (Variables|Default|GetProceduralMesh)))
  (Variables|三角形|Set三角形数量 (/ (Utilities|Array|Length _triangles) 3))
  (Variables|顶点|SetVertices _vertices)
  (Variables|Default|SetUVs _uvs)
  (Variables|Default|SetTriangles _triangles)
  ;[1 1 1] 遍历每个三角形(从 0 开始，三个一组)
  (for _index (range 0 (- (Variables|三角形|Get三角形数量) 1))
    (Variables|三角形|SetTri_A_Index (Utilities|Array|Get(acopy) (Variables|Default|GetTriangles) (+ (* _index 3) 0)))
    (Variables|三角形|SetTri_B_Index (Utilities|Array|Get(acopy) (Variables|Default|GetTriangles) (+ (* _index 3) 1)))
    (Variables|三角形|SetTri_C_Index (Utilities|Array|Get(acopy) (Variables|Default|GetTriangles) (+ (* _index 3) 2)))
    (bind (_canvas _size _context) (Rendering|BeginDrawCanvastoRenderTarget "/Game/Render/ZBuffer/RT_ZBuffer.RT_ZBuffer"))
    (Variables|Default|SetSize _size)
    (Rendering|Material|SetVectorParameterValue (Variables|Default|GetZ%20Buffer%20Depth%20Painter) "Triangle A" (Math|Color|MakeColor (.X (Math|Vector2D|BreakVector2D (.ScreenLocation (CallFunction|WorldtoScreen (Math|Transform|InverseTransformLocation (Variables|Default|GetCameraTransform) (Math|Transform|TransformLocation (Variables|Default|GetStatic%20Mesh%20Relative%20Transform) (Utilities|Array|Get(acopy) (Variables|顶点|GetVertices) (Variables|三角形|GetTri_A_Index)))))))) (.Y (Math|Vector2D|BreakVector2D (.ScreenLocation (CallFunction|WorldtoScreen (Math|Transform|InverseTransformLocation (Variables|Default|GetCameraTransform) (Math|Transform|TransformLocation (Variables|Default|GetStatic%20Mesh%20Relative%20Transform) (Utilities|Array|Get(acopy) (Variables|顶点|GetVertices) (Variables|三角形|GetTri_A_Index)))))))) (.X (Math|Vector2D|BreakVector2D (Utilities|Array|Get(acopy) (Variables|Default|GetUVs) (Variables|三角形|GetTri_A_Index)))) (.Y (Math|Vector2D|BreakVector2D (Utilities|Array|Get(acopy) (Variables|Default|GetUVs) (Variables|三角形|GetTri_A_Index))))) :!class /Script/Engine.MaterialInstanceDynamic)
    (Rendering|Material|SetVectorParameterValue (Variables|Default|GetZ%20Buffer%20Depth%20Painter) "Triangle B" (Math|Color|MakeColor (.X (Math|Vector2D|BreakVector2D (.ScreenLocation (CallFunction|WorldtoScreen (Math|Transform|InverseTransformLocation (Variables|Default|GetCameraTransform) (Math|Transform|TransformLocation (Variables|Default|GetStatic%20Mesh%20Relative%20Transform) (Utilities|Array|Get(acopy) (Variables|顶点|GetVertices) (Variables|三角形|GetTri_B_Index)))))))) (.Y (Math|Vector2D|BreakVector2D (.ScreenLocation (CallFunction|WorldtoScreen (Math|Transform|InverseTransformLocation (Variables|Default|GetCameraTransform) (Math|Transform|TransformLocation (Variables|Default|GetStatic%20Mesh%20Relative%20Transform) (Utilities|Array|Get(acopy) (Variables|顶点|GetVertices) (Variables|三角形|GetTri_B_Index)))))))) (.X (Math|Vector2D|BreakVector2D (Utilities|Array|Get(acopy) (Variables|Default|GetUVs) (Variables|三角形|GetTri_B_Index)))) (.Y (Math|Vector2D|BreakVector2D (Utilities|Array|Get(acopy) (Variables|Default|GetUVs) (Variables|三角形|GetTri_B_Index))))) :!class /Script/Engine.MaterialInstanceDynamic)
    (Rendering|Material|SetVectorParameterValue (Variables|Default|GetZ%20Buffer%20Depth%20Painter) "Triangle C" (Math|Color|MakeColor (.X (Math|Vector2D|BreakVector2D (.ScreenLocation (CallFunction|WorldtoScreen (Math|Transform|InverseTransformLocation (Variables|Default|GetCameraTransform) (Math|Transform|TransformLocation (Variables|Default|GetStatic%20Mesh%20Relative%20Transform) (Utilities|Array|Get(acopy) (Variables|顶点|GetVertices) (Variables|三角形|GetTri_C_Index)))))))) (.Y (Math|Vector2D|BreakVector2D (.ScreenLocation (CallFunction|WorldtoScreen (Math|Transform|InverseTransformLocation (Variables|Default|GetCameraTransform) (Math|Transform|TransformLocation (Variables|Default|GetStatic%20Mesh%20Relative%20Transform) (Utilities|Array|Get(acopy) (Variables|顶点|GetVertices) (Variables|三角形|GetTri_C_Index)))))))) (.X (Math|Vector2D|BreakVector2D (Utilities|Array|Get(acopy) (Variables|Default|GetUVs) (Variables|三角形|GetTri_C_Index)))) (.Y (Math|Vector2D|BreakVector2D (Utilities|Array|Get(acopy) (Variables|Default|GetUVs) (Variables|三角形|GetTri_C_Index))))) :!class /Script/Engine.MaterialInstanceDynamic)
    (Rendering|Material|SetVectorParameterValue (Variables|Default|GetZ%20Buffer%20Depth%20Painter) "InvDepth" (/ (Utilities|Struct|MakeLinearColor 1.0 1.0 1.0 1.0) (Math|Color|MakeColor (.Depth (CallFunction|WorldtoScreen (Math|Transform|InverseTransformLocation (Variables|Default|GetCameraTransform) (Math|Transform|TransformLocation (Variables|Default|GetStatic%20Mesh%20Relative%20Transform) (Utilities|Array|Get(acopy) (Variables|顶点|GetVertices) (Variables|三角形|GetTri_A_Index)))))) (.Depth (CallFunction|WorldtoScreen (Math|Transform|InverseTransformLocation (Variables|Default|GetCameraTransform) (Math|Transform|TransformLocation (Variables|Default|GetStatic%20Mesh%20Relative%20Transform) (Utilities|Array|Get(acopy) (Variables|顶点|GetVertices) (Variables|三角形|GetTri_B_Index)))))) (.Depth (CallFunction|WorldtoScreen (Math|Transform|InverseTransformLocation (Variables|Default|GetCameraTransform) (Math|Transform|TransformLocation (Variables|Default|GetStatic%20Mesh%20Relative%20Transform) (Utilities|Array|Get(acopy) (Variables|顶点|GetVertices) (Variables|三角形|GetTri_C_Index)))))))) :!class /Script/Engine.MaterialInstanceDynamic)
    ;[1 1 1] 渲染目标上绘制三角形
    (Class|Canvas|DrawMaterialTriangle _canvas (Variables|Default|GetZ%20Buffer%20Depth%20Painter) (Utilities|Array|MakeArray (Utilities|Struct|MakeCanvasUVTri (* (Variables|Default|GetSize) (.ScreenLocation (CallFunction|WorldtoScreen (Math|Transform|InverseTransformLocation (Variables|Default|GetCameraTransform) (Math|Transform|TransformLocation (Variables|Default|GetStatic%20Mesh%20Relative%20Transform) (Utilities|Array|Get(acopy) (Variables|顶点|GetVertices) (Variables|三角形|GetTri_A_Index))))))) (.ScreenLocation (CallFunction|WorldtoScreen (Math|Transform|InverseTransformLocation (Variables|Default|GetCameraTransform) (Math|Transform|TransformLocation (Variables|Default|GetStatic%20Mesh%20Relative%20Transform) (Utilities|Array|Get(acopy) (Variables|顶点|GetVertices) (Variables|三角形|GetTri_A_Index)))))) "(R=1.000000,G=1.000000,B=1.000000,A=1.000000)" (* (Variables|Default|GetSize) (.ScreenLocation (CallFunction|WorldtoScreen (Math|Transform|InverseTransformLocation (Variables|Default|GetCameraTransform) (Math|Transform|TransformLocation (Variables|Default|GetStatic%20Mesh%20Relative%20Transform) (Utilities|Array|Get(acopy) (Variables|顶点|GetVertices) (Variables|三角形|GetTri_B_Index))))))) (.ScreenLocation (CallFunction|WorldtoScreen (Math|Transform|InverseTransformLocation (Variables|Default|GetCameraTransform) (Math|Transform|TransformLocation (Variables|Default|GetStatic%20Mesh%20Relative%20Transform) (Utilities|Array|Get(acopy) (Variables|顶点|GetVertices) (Variables|三角形|GetTri_B_Index)))))) "(R=1.000000,G=1.000000,B=1.000000,A=1.000000)" (* (Variables|Default|GetSize) (.ScreenLocation (CallFunction|WorldtoScreen (Math|Transform|InverseTransformLocation (Variables|Default|GetCameraTransform) (Math|Transform|TransformLocation (Variables|Default|GetStatic%20Mesh%20Relative%20Transform) (Utilities|Array|Get(acopy) (Variables|顶点|GetVertices) (Variables|三角形|GetTri_C_Index))))))) (.ScreenLocation (CallFunction|WorldtoScreen (Math|Transform|InverseTransformLocation (Variables|Default|GetCameraTransform) (Math|Transform|TransformLocation (Variables|Default|GetStatic%20Mesh%20Relative%20Transform) (Utilities|Array|Get(acopy) (Variables|顶点|GetVertices) (Variables|三角形|GetTri_C_Index)))))) "(R=1.000000,G=1.000000,B=1.000000,A=1.000000)")))
    (Rendering|EndDrawCanvastoRenderTarget _context)
    (Rendering|DrawMaterialtoRenderTarget "/Game/Render/ZBuffer/RT_ZBufferCopy.RT_ZBufferCopy" "/Game/Render/ZBuffer/M_ZBuffer.M_ZBuffer")))

(fn ConstructionScript)

(fn WorldtoScreen
  (params (WorldLocaiton :type Vector))
  (bind (_x _y _z) (Math|Vector|BreakVector WorldLocaiton))
  (bind _fov (Variables|Default|GetFOV))
  (bind _size (Variables|Default|GetSize))
  (bind _returnvalue (/ _fov 2.0))
  (bind _returnvalue_2 (Math|Trig|Tan(Degrees) _returnvalue))
  (return (+ (* (/ (Math|Vector2D|MakeVector2D _y _z) (* (Math|Vector2D|MakeVector2D _x _x) (* (Math|Vector2D|MakeVector2D _returnvalue_2 _returnvalue_2) (Math|Vector2D|MakeVector2D 1.0 (/ (.y _size) (.x _size)))))) "(X=0.500000,Y=-0.500000)") "(X=0.500000,Y=0.500000)") _x))