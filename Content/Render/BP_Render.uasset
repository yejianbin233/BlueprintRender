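; BP_Render is a simple software renderer that draws a cube's mesh into the RT_Depth render target once on BeginPlay.
; It copies the static mesh to a procedural mesh to read section 0's vertices, UVs and triangle indices.
; Each vertex moves through mesh-relative and inverse camera transforms, then WorldToScreen applies FOV and aspect-ratio perspective projection.
; Canvas DrawTriangle draws each triangle textured with CASC_Lights, without depth testing.
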(event EventBeginPlay
  (Rendering|ClearRenderTarget2D "/Game/Render/RT_Depth.RT_Depth")
  (Variables|Default|SetStatic%20Mesh%20Relative%20Transform (Transformation|GetRelativeTransform (Variables|Default|GetCube)))
  (Class|KismetProceduralMeshLibrary|CopyProceduralMeshfromStaticMeshComponent (Variables|Default|GetCube) 0 (Variables|Default|GetProceduralMesh) false)
  (bind (_vertices _triangles _normals _uvs) (Class|KismetProceduralMeshLibrary|GetSectionfromProceduralMesh (Variables|Default|GetProceduralMesh)))
  (Variables|三角形|Set三角形数量 (/ (Utilities|Array|Length _triangles) 3))
  (Variables|顶点|SetVertices _vertices)
  (Variables|Default|SetUVs _uvs)
  (Variables|Default|SetTriangles _triangles)
  (bind (_canvas _size _context) (Rendering|BeginDrawCanvastoRenderTarget "/Game/Render/RT_Depth.RT_Depth"))
  (Variables|Default|SetSize _size)
  ;[1 1 1] 遍历每个三角形(从 0 开始，三个一组)
  (for _index (range 0 (- (Variables|三角形|Get三角形数量) 1))
    (Variables|三角形|SetTri_A_Index (Utilities|Array|Get(acopy) (Variables|Default|GetTriangles) (+ (* _index 3) 0)))
    (Variables|三角形|SetTri_B_Index (Utilities|Array|Get(acopy) (Variables|Default|GetTriangles) (+ (* _index 3) 1)))
    (Variables|三角形|SetTri_C_Index (Utilities|Array|Get(acopy) (Variables|Default|GetTriangles) (+ (* _index 3) 2)))
    ;[1 1 1] 渲染目标上绘制三角形
    (Class|Canvas|DrawTriangle _canvas "/Engine/EditorMaterials/Cascade/CASC_Lights.CASC_Lights" (Utilities|Array|MakeArray (Utilities|Struct|MakeCanvasUVTri (* (Variables|Default|GetSize) (CallFunction|WorldtoScreen (Math|Transform|InverseTransformLocation (Variables|Default|GetCameraTransform) (Math|Transform|TransformLocation (Variables|Default|GetStatic%20Mesh%20Relative%20Transform) (Utilities|Array|Get(acopy) (Variables|顶点|GetVertices) (Variables|三角形|GetTri_A_Index)))))) (Utilities|Array|Get(acopy) (Variables|Default|GetUVs) (Variables|三角形|GetTri_A_Index)) "(R=1.000000,G=1.000000,B=1.000000,A=1.000000)" (* (Variables|Default|GetSize) (CallFunction|WorldtoScreen (Math|Transform|InverseTransformLocation (Variables|Default|GetCameraTransform) (Math|Transform|TransformLocation (Variables|Default|GetStatic%20Mesh%20Relative%20Transform) (Utilities|Array|Get(acopy) (Variables|顶点|GetVertices) (Variables|三角形|GetTri_B_Index)))))) (Utilities|Array|Get(acopy) (Variables|Default|GetUVs) (Variables|三角形|GetTri_B_Index)) "(R=1.000000,G=1.000000,B=1.000000,A=1.000000)" (* (Variables|Default|GetSize) (CallFunction|WorldtoScreen (Math|Transform|InverseTransformLocation (Variables|Default|GetCameraTransform) (Math|Transform|TransformLocation (Variables|Default|GetStatic%20Mesh%20Relative%20Transform) (Utilities|Array|Get(acopy) (Variables|顶点|GetVertices) (Variables|三角形|GetTri_C_Index)))))) (Utilities|Array|Get(acopy) (Variables|Default|GetUVs) (Variables|三角形|GetTri_C_Index)) "(R=1.000000,G=1.000000,B=1.000000,A=1.000000)"))))
  (Rendering|EndDrawCanvastoRenderTarget _context))

(fn ConstructionScript)

(fn WorldtoScreen
  (params (WorldLocaiton :type Vector))
  (bind (_x _y _z) (Math|Vector|BreakVector WorldLocaiton))
  (bind _fov (Variables|Default|GetFOV))
  (bind _size (Variables|Default|GetSize))
  (bind _returnvalue (/ _fov 2.0))
  (bind _returnvalue_2 (Math|Trig|Tan(Degrees) _returnvalue))
  (return (+ (* (/ (Math|Vector2D|MakeVector2D _y _z) (* (Math|Vector2D|MakeVector2D _x _x) (* (Math|Vector2D|MakeVector2D _returnvalue_2 _returnvalue_2) (Math|Vector2D|MakeVector2D 1.0 (/ (.y _size) (.x _size)))))) "(X=0.500000,Y=-0.500000)") "(X=0.500000,Y=0.500000)")))